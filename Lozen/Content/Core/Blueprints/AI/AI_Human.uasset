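; AI controller for human characters that reacts to enemies it sees or hears.
; Sight locks the pawn onto a new enemy, toggles weapon and attack mode via messages and moves toward it, while hearing moves toward enemy stimuli.
; GotoLocation throttles moves with a DoOnce and delay.
; GetTargetLocation picks a reachable intermediate point for distant targets, but returns a zero vector for near ones.
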(event `self.ReceiveBeginPlay`
  ;[0 0.2232 0.5029] Set AI Pawn Variable
  (set `self.AIPawn` (`self.K2_GetPawn`)))

(event `self.GoToLocation`
  (params (`Target Location` :type "Vector Structure"))
  (bind _randomlocation (`self.GetTargetLocation` `Target Location`))
  ;[1 0.4994 0] Go To Location
  (set `self.MoveDestination` `Target Location`)
  (`/Engine/EditorBlueprintResources/StandardMacros.DoOnce` false :!label _label
    (:`Completed`
      (`self.MoveToLocation` _randomlocation 10.0 true true true true null)
      (if (< (`self.GetDistanceAndDirection` _randomlocation (`self.K2_GetActorLocation` (`self.AIPawn`))) 200.0)
        (goto _label :!via `Reset`)
        (else
          (`self.MoveToLocation` _randomlocation 10.0 true true true true null)
          (`KismetSystemLibrary.Delay` 10.0)
          (goto _label :!via `Reset`))))))

(fn `GetDistanceAndDirection`
  (params (`Target Location` :type "Vector Structure") (`Current Location` :type "Vector Structure"))
  (returns (Distance :type "Float (double-precision)") (Direction :type "Vector Structure"))
  (bind _returnvalue (- `Target Location` `Current Location`))
  (return (`KismetMathLibrary.VSize` _returnvalue) (`KismetMathLibrary.Normal` _returnvalue)))

(fn `GetTargetLocation`
  (params (Origin :type "Vector Structure (by ref)"))
  (returns (RandomLocation :type "Vector Structure"))
  (bind _returnvalue (`self.K2_GetActorLocation` (`self.AIPawn`)))
  (bind (_distance _direction) (`self.GetDistanceAndDirection` (`NavigationSystemV1.K2_GetRandomReachablePointInRadius` Origin 100.0 null null) _returnvalue))
  ;[1 0 0.008603] IF distance between pawn and target location is smaller than 2500
  (if (< _distance 2500.0)
    (return (0.0 0.0 0.0))
    (else
      (return (`NavigationSystemV1.K2_GetRandomReachablePointInRadius` (+ _returnvalue (* _direction 1500.0)) 100.0 null null)))))

(fn `OnAIAlert?`
  (returns (`Alert?` :type Boolean))
  (return (`self.Seen`)))

(fn `UserConstructionScript`)