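; BP_Weapon is a melee sword actor that supplies its attack montages, visual effects and socket transforms.
; Montage getters cycle through regular or combo attack arrays by attack count and also return a charge attack.
; A dynamic blade material created on BeginPlay drives the charge effect, while the trail plays as a looping mesh animation stopped after a delay.
; Detaching turns on blocking collision and physics simulation so the weapon falls free.
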(event `self.ReceiveBeginPlay`
  (bind _returnvalue (`PrimitiveComponent.CreateDynamicMaterialInstance` (`self.WeaponMesh`) 0 "/Game/InfinityBladeWeapons/Weapons/Blade/Swords/Blade_HeroSword10/M_Blade_HeroSword.M_Blade_HeroSword" "None"))
  (set `self.WeaponMaterial` _returnvalue))

(event `/Game/Core/Blueprints/Weapons/BPI_Weapon.DetachWeapon`
  (bind _weaponmesh (`self.WeaponMesh`))
  (`PrimitiveComponent.SetCollisionEnabled` _weaponmesh "PhysicsOnly")
  (`PrimitiveComponent.SetCollisionProfileName` _weaponmesh "BlockAll")
  (`PrimitiveComponent.SetSimulatePhysics` _weaponmesh true))

(event `/Game/Core/Blueprints/Weapons/BPI_Weapon.ActivateSwordTrail`
  (params (Duration :type "Float (single-precision)"))
  (bind _weaponmesh (`self.WeaponMesh`))
  (`SkeletalMeshComponent.PlayAnimation` _weaponmesh (`self.SwordTrailAnim`) true)
  (`KismetSystemLibrary.Delay` Duration)
  (`SkeletalMeshComponent.Stop` _weaponmesh))

(event `/Game/Core/Blueprints/Weapons/BPI_Weapon.ToggleChargeWeapon`
  (params (`Enabled?` :type Boolean))
  (`MaterialInstanceDynamic.SetScalarParameterValue` (`self.WeaponMaterial`) "Charge Multiplier" (select `bool` `Enabled?` :`true` 10.0 :!type "Float (single-precision)")))

(fn `GetAttackMontage`
  (params (AttackCount :type Integer) (IsComboAttack :type Boolean))
  (returns (AttackMontage :type "AnimMontage Object Reference"))
  (bind _regularattacks (`self.RegularAttacks`))
  (bind _comboattacks (`self.ComboAttacks`))
  (if IsComboAttack
    (return (`|GetArrayItem` _comboattacks (mod AttackCount (`KismetArrayLibrary.Array_Length` _comboattacks))))
    (else
      (return (`|GetArrayItem` _regularattacks (mod AttackCount (`KismetArrayLibrary.Array_Length` _regularattacks)))))))

(fn `GetChargeMontage`
  (returns (`Charge Montage` :type "AnimMontage Object Reference"))
  (return (`self.ChargeAttack`)))

(fn `GetWeaponSocketTransform`
  (params (SocketName :type Name))
  (returns (Transform :type "Transform Structure"))
  (return (`SceneComponent.GetSocketTransform` (`self.WeaponMesh`) SocketName "RTS_World")))

(fn `UserConstructionScript`)