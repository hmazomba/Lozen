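; Enemy AI character that fights a locked target in melee-style rounds and shows its health on an overhead-style widget.
; Attack mode uses a looping FlipFlop to alternate randomly timed attack phases with strafe phases that randomly toggle blocking.
; The attack loop closes to hit range, queries the target through message calls, and flashes a warning for randomly charged or normal attacks.
; Tick refreshes health and, outside attacks, strafes while holding distance from the target.
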(event `self.ReceiveBeginPlay`
  (`parent.ReceiveBeginPlay`)
  (`self.UpdateActorDetails`))

(event `self.ReceiveTick`
  (params (DeltaSeconds :type "Float (single-precision)"))
  (bind _returnvalue (`KismetMathLibrary.MakeRotator` 0.0 0.0 (.yaw (`self.GetControlRotation`))))
  (`parent.ReceiveTick` DeltaSeconds)
  (`self.UpdateActorDetails`)
  (`/Engine/EditorBlueprintResources/StandardMacros.IsValid` (`self.LockedEnemy`)
    (:`Is Valid`
      (if (not (`self.IsAttacking`))
        (`self.AddMovementInput` (`KismetMathLibrary.GetRightVector` _returnvalue) (`self.CombatStrafe`))
        (`self.AddMovementInput` (`KismetMathLibrary.GetForwardVector` _returnvalue) (select `bool` (> (`self.GetDistanceTo` (`self.LockedEnemy`) self) 600.0) :`false` -0.5 :`true` 0.5 :!type "Float (single-precision)"))))))

(event `self.ToggleAttacking`
  (params (Enable :type Boolean) (Enemy :type "Actor Object Reference"))
  (bind _returnvalue (`self.K2_GetActorLocation` Enemy))
  ;[0.9922 0 1] NPC Attack loop
  (bind _output_get (set `self.IsAttacking` Enable))
  (if _output_get
    (`/Engine/EditorBlueprintResources/StandardMacros.DoOnce` false :!label _label
      (:`Completed`
        (`/Engine/EditorBlueprintResources/StandardMacros.IsValid` Enemy :!label _label_2
          (:`Is Valid`
            _)
          (:`Is Not Valid`
            (`self.GetClosestEnemy`)))
        (if (< (`self.GetDistanceTo` Enemy self) (`self.HitRange`)) :!label _label_3
          (bind _alive_ (message `/Game/Core/Blueprints/Characters/BPI_Character.IsAlive?` Enemy))
          (if _alive_
            (bind _underattack_ (message `/Game/Core/Blueprints/Characters/BPI_Character.IsUnderAttack?` Enemy 0.5 self))
            (else
              (`self.ToggleAttackMode` false)))
          (if _underattack_
            _
            (elif (`self.IsReadyForNextAnim?`)
              (bind _output_get_2 (set `self.IsCharged?` (`KismetMathLibrary.RandomBool`)))
              (message `/Game/Core/Blueprints/UI/BPI_UI.ShowText` (`WidgetComponent.GetUserWidgetObject` (`self.Widget`)) 0.8 (select `bool` _output_get_2 :`false` "INCOMING!!!" :`true` "DANGER!!!" :!type "Text") (select `bool` _output_get_2 :`false` (make `SlateColor` (struct :`R` 1.0 :`G` 0.937491 :`B` 0.297666 :`A` 1.0)) :`true` (make `SlateColor` (struct :`R` 1.0 :`A` 1.0))))
              (`self.AIAttack`)))
          (`KismetSystemLibrary.Delay` (`KismetMathLibrary.RandomFloatInRange` 2.5 5.0))
          (if (and (`self.IsAttacking`) (not (`self.IsDead`)))
            (goto _label_2)
            (else
              (goto _label :!via `Reset`)))
          (else
            (`AIController.MoveToLocation` (`AIBlueprintHelperLibrary.GetAIController` self) (+ (* (`KismetMathLibrary.Normal` (- (`self.K2_GetActorLocation`) _returnvalue)) (* (`self.HitRange`) 0.5)) _returnvalue) 10.0 true true false true null false)
            (`KismetSystemLibrary.Delay` 1.0)
            (goto _label_3)))))))

(event `self.ToggleAttackMode`
  (params (Enable :type Boolean) (Enemy :type "Actor Object Reference"))
  (set `self.LockedEnemy` Enemy)
  (bind _output_get (set `self.InAttackMode?` Enable))
  (if _output_get
    (`/Engine/EditorBlueprintResources/StandardMacros.DoOnce` false :!label _label_4
      (:`Completed`
        (`/Engine/EditorBlueprintResources/StandardMacros.FlipFlop` :!label _label_5
          (:`A`
            ;[0 1 0.3906] AI Attack
            (set `self.CombatStrafe` 0.0)
            (`self.ToggleAttacking` true (`self.LockedEnemy`))
            (`KismetSystemLibrary.Delay` (`KismetMathLibrary.RandomFloatInRange` 4.0 10.0)))
          (:`B`
            (`self.ToggleBlock` (`KismetMathLibrary.RandomBool`))
            ;[0 1 0.3672] Strafe
            (set `self.CombatStrafe` (`KismetMathLibrary.RandomFloatInRange` -0.3 0.3))
            (`self.ToggleAttacking` false)
            (`KismetSystemLibrary.Delay` (`KismetMathLibrary.RandomFloatInRange` 4.0 10.0))))
        (if (`self.InAttackMode?`)
          (goto _label_5)
          (else
            (goto _label_4 :!via `Reset`)))))
    (else
      (`self.ToggleAttacking` false)
      (`self.LockOn` null))))

(event `self.UpdateActorDetails`
  (message `/Game/Core/Blueprints/UI/BPI_UI.UpdateNumber` (`WidgetComponent.GetUserWidgetObject` (`self.Widget`)) (/ (`self.Health`) (`self.MaxHealth`))))

(fn `Alerted?`
  (returns (`Alert?` :type Boolean))
  (bind _alert_ (message `/Game/Core/Blueprints/AI/BPI_AI.OnAIAlert?` (`self.GetController`)))
  (return _alert_))

(fn `UserConstructionScript`
  (`parent.UserConstructionScript`))