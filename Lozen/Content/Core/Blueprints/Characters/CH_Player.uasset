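; Player character Blueprint adding stealth takedowns, combat camera behavior and notification UI.
; A box overlap stores an unalerted enemy and shows a tip; the Takedown input turns to it, readies a weapon and plays a montage, with damage applied in a Takedown event.
; Tick eases spring-arm length, widened while under attack, and interpolates control rotation while an attacker is set.
; Enemy death triggers brief slow motion.
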(event `self.ReceiveBeginPlay`
  (`parent.ReceiveBeginPlay`)
  (bind _returnvalue (`|CreateWidget` "/Game/Core/Blueprints/UI/Widg_Notification.Widg_Notification_C" (`GameplayStatics.GetPlayerController` 0)))
  (bind _output_get (set `self.Widg_Notifications` _returnvalue))
  (`UserWidget.AddToViewport` _output_get 0))

(event `self.ReceiveTick`
  (params (DeltaSeconds :type "Float (single-precision)"))
  (bind _returnvalue (`self.GetController`))
  (bind _targetspringarmlength (`self.TargetSpringArmLength`))
  (bind _cameraboom (`self.CameraBoom`))
  (bind _targetfov (`self.TargetFOV`))
  (bind _followcamera (`self.FollowCamera`))
  (bind _targetarmlength (`SpringArmComponent.TargetArmLength` _cameraboom))
  (bind _fieldofview (`CameraComponent.FieldOfView` _followcamera))
  (`parent.ReceiveTick` DeltaSeconds)
  (if (!= _targetspringarmlength _targetarmlength)
    (set `SpringArmComponent.TargetArmLength` (`KismetMathLibrary.Lerp` _targetarmlength _targetspringarmlength 0.1) _cameraboom))
  (if (!= _targetfov _fieldofview)
    (`CameraComponent.SetFieldOfView` _followcamera (`KismetMathLibrary.Lerp` _fieldofview _targetfov)))
  (`/Engine/EditorBlueprintResources/StandardMacros.IsValid` (`self.Attacker`)
    (:`Is Valid`
      (`Controller.SetControlRotation` _returnvalue (`KismetMathLibrary.RInterpTo` (`Controller.GetControlRotation` _returnvalue) (`self.TargetRotation`) 0.5 0.5)))
    (:`Is Not Valid`)))

(event `self.Box.OnComponentBeginOverlap`
  (params (OverlappedComponent :type "PrimitiveComponent Object Reference") (OtherActor :type "Actor Object Reference") (OtherComp :type "PrimitiveComponent Object Reference") (OtherBodyIndex :type Integer) (bFromSweep :type Boolean) (SweepResult :type "HitResult Structure (by ref)"))
  (bind _yes_no (message `/Game/Core/Blueprints/Characters/BPI_Character.IsEnemy` OtherActor (`self.Team`)))
  (bind _alert_ (message `/Game/Core/Blueprints/Characters/BPI_Character.Alerted?` OtherActor))
  (if (and (not _alert_) _yes_no)
    (set `self.TakedownEnemy` OtherActor)
    (`/Game/Core/Blueprints/UI/BPI_UI.ShowTip` (`self.Widg_Notifications`) "Press 'F' to Takedown" 3.0)))

(event `InputAction|Takedown`
  (params (Key :type "Key Structure"))
  (bind _takedownenemy (`self.TakedownEnemy`))
  (:`Pressed`
    (`/Engine/EditorBlueprintResources/StandardMacros.IsValid` _takedownenemy
      (:`Is Valid`
        (`self.RotateToActor_M` _takedownenemy
          (:`exec`
            (if (not (> (`self.CurrentWeaponIndex`) 0))
              (`/Game/Core/Blueprints/Characters/BPI_Character.ToggleWeapon` true)
              (`KismetSystemLibrary.Delay` 0.2))
            (`self.PlayAnimMontage` "/Game/Core/Characters/Eva/Animations/Combat/AM_Takedown.AM_Takedown")))))))

(event `/Game/Core/Blueprints/Characters/BPI_Character.Takedown`
  (message `/Game/Core/Blueprints/Characters/BPI_Character.DealDamage` (`self.TakedownEnemy`) 100.0))

(event `/Game/Core/Blueprints/Characters/BPI_Character.SetAnimRateScale`
  (params (RateScale :type "Float (single-precision)")))

(event `self.SetUnderAttack`
  (params (Duration :type "Float (single-precision)") (Attacker :type "Actor Object Reference"))
  (`parent.SetUnderAttack` Duration Attacker)
  (set `self.TargetRotation` (`KismetMathLibrary.FindLookAtRotation` (`self.K2_GetActorLocation`) (`self.K2_GetActorLocation`)))
  (set `self.Attacker` Attacker)
  (`KismetSystemLibrary.Delay` Duration)
  (set `self.Attacker` null))

(event `/Game/Core/Blueprints/Characters/BPI_Character.OnEnemyDeath`
  (`GameplayStatics.SetGlobalTimeDilation` 0.1)
  (`KismetSystemLibrary.Delay` 0.5)
  (`GameplayStatics.SetGlobalTimeDilation` 1.0))

(event `self.ToggleFightCamera`
  (params (Enable :type Boolean))
  (set `self.TargetSpringArmLength` (select `bool` Enable :`false` 300.0 :`true` 500.0 :!type "Float (single-precision)")))

(event `self.ChangeCameraParameters`
  (params (SpringArmLength :type "Float (single-precision)") (FOV :type "Float (single-precision)"))
  (set `self.TargetSpringArmLength` SpringArmLength)
  (set `self.TargetFOV` FOV))

(fn `IsUnderAttack?`
  (params (AttackDuration :type "Float (double-precision)") (Attacker :type "Actor Object Reference"))
  (returns (`UnderAttack?` :type Boolean))
  (bind _underattack_ (`parent.IsUnderAttack?` AttackDuration Attacker))
  (`self.ToggleFightCamera` _underattack_)
  (return _underattack_))

(fn `UserConstructionScript`
  (`parent.UserConstructionScript`))